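; BP_EnemySpawn is a one-shot spawner that creates an enemy squad when BP_MainCharacter enters its trigger sphere.
; The construction script sizes the TriggerArea and SpawnArea spheres from their range variables.
; On overlap it rolls a squad size, spawns EnemyType pawns running BT_EnemyAI, then destroys itself.
; Random X and Y offsets run from zero to SpawnRange, so enemies land in a positive-quadrant square rather than the SpawnArea sphere.
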(event OnComponentBeginOverlap(TriggerArea)
  (params (OverlappedComponent :type Primitive%20Component%20Object%20Reference) (OtherActor :type Actor%20Object%20Reference) (OtherComp :type Primitive%20Component%20Object%20Reference) (OtherBodyIndex :type Integer) (bFromSweep :type Boolean) (SweepResult :type Hit%20Result%20Structure%20%28by%20ref%29))
  ;[0 0 0] Core
  (Utilities|Casting|CastToBP_MainCharacter OtherActor)
  (CallFunction|SetupSpawner)
  (CallFunction|SetupEnemies)
  (Actor|DestroyActor))

(fn ConstructionScript
  (Components|Sphere|SetSphereRadius (Variables|Default|GetTriggerArea) (Variables|Spawning|GetTriggerRange) true)
  (Components|Sphere|SetSphereRadius (Variables|Default|GetSpawnArea) (Variables|Spawning|GetSpawnRange) true))

(fn SetupEnemies
  (bind _returnvalue (Transformation|GetActorTransform))
  (bind (_location _rotation) (Math|Transform|BreakTransform _returnvalue))
  (for _index (range 1 (Variables|Spawning|GetSquadSize))
    (bind _newspawnposition (CallFunction|RandomizeLocation _location (Variables|Spawning|GetSpawnRange)))
    (AI|SpawnAIFromClass (Variables|Spawning|GetEnemyType) "/Game/Blueprints/Characters/EnemyDummy/BT_EnemyAI.BT_EnemyAI" _newspawnposition _rotation false)))

(fn RandomizeLocation
  (params (SpawnLocation :type Vector) (Range :type Float%20%28single-precision%29))
  (return (+ SpawnLocation (Math|Vector|MakeVector (Math|Random|RandomFloatinRange 0.0 Range) (Math|Random|RandomFloatinRange 0.0 Range) 0.0))))

(fn SetupSpawner
  (Variables|Spawning|SetSquadSize (Math|Random|RandomIntegerinRange (Variables|Spawning|GetMinSqaudSize) (Variables|Spawning|GetMaxSquadSize))))