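; BP_PointOfInterest is a level generator spawner that places one random structure at its own transform when play begins.
; SetupStructures expands the Spawnables map into a weighted Structures array, using each integer key as the number of copies of its class.
; SpawnStructure picks a uniformly random entry from that array, spawns it with adjust-if-possible-but-always-spawn collision handling, and prints the result.
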(event EventBeginPlay
  (CallFunction|SetupStructures)
  (CallFunction|SpawnStructure))

(fn ConstructionScript)

(fn SpawnStructure
  (bind _structures (Variables|Spawning|GetStructures))
  (bind _returnvalue (Game|SpawnActorfromClass (Utilities|Array|Get(acopy) _structures (Math|Random|RandomIntegerinRange 0 (- (Utilities|Array|Length _structures) 1))) (Transformation|GetActorTransform) "AdjustIfPossibleButAlwaysSpawn" 0 0))
  (Development|PrintText (Utilities|Text|ToText(Object) _returnvalue)))

(fn SetupStructures
  (bind _spawnables (Variables|Spawning|GetSpawnables))
  (bind _keys (Utilities|Map|Keys _spawnables))
  (bind _values (Utilities|Map|Values _spawnables))
  (for (_array_element _array_index) _keys
    (for _index (range 1 _array_element)
      (Utilities|Array|Add (Variables|Spawning|GetStructures) (Utilities|Array|Get(acopy) _values _array_index)))))