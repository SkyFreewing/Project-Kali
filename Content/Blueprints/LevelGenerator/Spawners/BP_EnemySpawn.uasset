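; Enemy spawner for the level generator that creates a random-sized AI squad when the main character enters its trigger sphere.
; Spawning requires an unclamped per-tick countdown to equal exactly zero, and happens once unless EndlessSpawning is set.
; Enemies run BT_EnemyAI and receive the shared squad, home spawner and their offset from it.
; It also builds random reachable patrol waypoints, served cyclically by GetNextWaypoint.
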(event OnComponentBeginOverlap(TriggerArea)
  (params (OverlappedComponent :type Primitive%20Component%20Object%20Reference) (OtherActor :type Actor%20Object%20Reference) (OtherComp :type Primitive%20Component%20Object%20Reference) (OtherBodyIndex :type Integer) (bFromSweep :type Boolean) (SweepResult :type Hit%20Result%20Structure%20%28by%20ref%29))
  ;[0 0 0] Core
  (if (== (Variables|Default|GetTimeToSpawn) 0)
    (Utilities|Casting|CastToBP_MainCharacter OtherActor)
    (if (not (Variables|KI|GetSpawned))
      (CallFunction|SetupSpawner)
      (CallFunction|SetupEnemies)
      (CallFunction|CreateRoute)
      (Variables|Default|SetTimeToSpawn 30))))

(event EventTick
  (params (DeltaSeconds :type Float%20%28single-precision%29))
  (Math|Integer|DecrementInt (Variables|Default|GetTimeToSpawn)))

(fn ConstructionScript
  (Components|Sphere|SetSphereRadius (Variables|Default|GetTriggerArea) (Variables|Spawning|GetTriggerRange) true)
  (Components|Sphere|SetSphereRadius (Variables|Default|GetSpawnArea) (Variables|Spawning|GetSpawnRange) true))

(fn SetupEnemies
  (bind _returnvalue (Transformation|GetActorTransform))
  (bind _returnvalue_2 (Transformation|GetActorLocation))
  (bind (_location _rotation) (Math|Transform|BreakTransform _returnvalue))
  (for _index (range 1 (Variables|Spawning|GetSquadSize))
    ;[1 1 1] Spawn Enemies + Add them to Squad
    (bind _newspawnposition (CallFunction|RandomizeLocation _location (Variables|Spawning|GetSpawnRange)))
    (bind _returnvalue_3 (AI|SpawnAIFromClass (Variables|Spawning|GetEnemyType) "/Game/Blueprints/Characters/EnemyDummy/BT_EnemyAI.BT_EnemyAI" _newspawnposition _rotation false))
    (bind _asbp_dummy_enemy (Utilities|Casting|CastToBP_DummyEnemy _returnvalue_3))
    (Utilities|Array|Add (Variables|KI|GetSquad) _asbp_dummy_enemy))
  (for _array_element (Variables|KI|GetSquad)
    (Variables|/Game/Blueprints/Characters/EnemyDummy/BP_DummyEnemy.BP_DummyEnemy_C|SetSquad _array_element (Variables|KI|GetSquad))
    (Variables|/Game/Blueprints/Characters/EnemyDummy/BP_DummyEnemy.BP_DummyEnemy_C|SetHome _array_element self)
    (Variables|/Game/Blueprints/Characters/EnemyDummy/BP_DummyEnemy.BP_DummyEnemy_C|SetOffset _array_element (* (Math|Vector|GetUnitDirection(Vector) _returnvalue_2 (Transformation|GetActorLocation _array_element)) (Math|Vector|Distance(Vector) _returnvalue_2 (Transformation|GetActorLocation _array_element))))))

(fn RandomizeLocation
  (params (SpawnLocation :type Vector) (Range :type Float%20%28single-precision%29))
  (return (+ SpawnLocation (Math|Vector|MakeVector (Math|Random|RandomFloatinRange 0.0 Range) (Math|Random|RandomFloatinRange 0.0 Range) 0.0))))

(fn SetupSpawner
  (if (Variables|Default|GetEndless%20Spawning!)
    _
    (else
      (Variables|KI|SetSpawned true)))
  (Variables|Spawning|SetSquadSize (Math|Random|RandomIntegerinRange (Variables|Spawning|GetMinSqaudSize) (Variables|Spawning|GetMaxSquadSize))))

(fn CreateRoute
  (for _index (range 0 5)
    (Utilities|Array|Add (Variables|KI|GetWaypoints) (.RandomLocation (AI|Navigation|GetRandomReachablePointinRadius (Transformation|GetActorLocation) (Variables|KI|GetPatrolRadius) 0 0)))))

(fn GetNextWaypoint
  (bind _waypoints (Variables|KI|GetWaypoints))
  (bind _result (Math|Integer|IncrementInt (Variables|KI|GetWaypointIndex))
    (:%20%20
      (if (>= _result (Utilities|Array|Length _waypoints))
        (Variables|KI|SetWaypointIndex 0))
      (return (Utilities|Array|Get(acopy) _waypoints (Variables|KI|GetWaypointIndex))))))