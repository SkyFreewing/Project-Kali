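; BP_Shrine_Ability is an arena shrine that grants the player a random ability, usable once.
; It extends a parent shrine, running parent logic on begin play and trigger.
; An aura particle shows while the shrine is active, either from begin play or after ActivateShrine clears the inactive state.
; Triggering an active, unused shrine marks it used, asks the GameManager for the ability and swaps the aura to a reaction effect.
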(event Custom|Event%20ActivateShrine
  (Rendering|SetVisibility (Variables|Default|GetPS_TriggerAura) true false)
  (Variables|Core|SetInactive false))

(event EventBeginPlay
  (|CallParentFunction)
  (if (not (Variables|Core|GetInactive))
    (Rendering|SetVisibility (Variables|Default|GetPS_TriggerAura) true false)))

(event EventTriggerShrine
  (|CallParentFunction)
  (if (not (or (Variables|Default|GetUsed) (Variables|Core|GetInactive)))
    (Variables|Default|SetUsed true)
    (Default|AddRandomAbilitytoPlayer (Variables|Default|GetGameManager))
    (CallFunction|PlayCollectedPS)))

(fn ConstructionScript
  (|CallParentFunction))

(fn PlayCollectedPS
  (Effects|Components|ParticleSystem|SetTemplate (Variables|Default|GetPS_TriggerAura) "/Game/VFX/particles/p_ShrineReact.p_ShrineReact"))