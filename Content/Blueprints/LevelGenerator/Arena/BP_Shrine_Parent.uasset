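; BP_Shrine_Parent is the base class for arena shrines that trigger when the main character enters their range.
; The construction script configures the trigger sphere's offset and radius plus the aura particle's scale, activation and visibility from variables.
; BeginPlay caches the game manager; on overlap it takes the character's sound manager and calls TriggerShrine.
; TriggerShrine and Reset are empty here, apparently hooks for child shrines.
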(event OnComponentBeginOverlap(TriggerRange)
  (params (OverlappedComponent :type Primitive%20Component%20Object%20Reference) (OtherActor :type Actor%20Object%20Reference) (OtherComp :type Primitive%20Component%20Object%20Reference) (OtherBodyIndex :type Integer) (bFromSweep :type Boolean) (SweepResult :type Hit%20Result%20Structure%20%28by%20ref%29))
  (bind _asbp_main_character (Utilities|Casting|CastToBP_MainCharacter OtherActor))
  (Variables|Core|SetSoundManager (Variables|/Game/Blueprints/Characters/MainCharacter/BP_MainCharacter.BP_MainCharacter_C|GetSound%20Manager _asbp_main_character))
  (Core|TriggerShrine))

(event EventBeginPlay
  (Core|GetGameManager))

(fn ConstructionScript
  (Transformation|SetRelativeLocation (Variables|Default|GetTriggerRange) (Variables|Core|GetTriggerOffset) false false)
  (Components|Sphere|SetSphereRadius (Variables|Default|GetTriggerRange) (Variables|Core|GetTrigger%20Radius) true)
  (Transformation|SetRelativeScale3D (Variables|Default|GetPS_TriggerAura) (Variables|Core|GetParticleScale))
  (Components|Activation|SetAutoActivate (Variables|Default|GetPS_TriggerAura) (Variables|Core|GetActive))
  (Rendering|SetVisibility (Variables|Default|GetPS_TriggerAura) (Variables|Core|GetIsVisible) true))

(fn GetGameManager
  (bind _outactors (Actor|GetAllActorsOfClass "/Game/Blueprints/Management/BP_GameManager.BP_GameManager_C"))
  (Variables|Core|SetGameManager (Utilities|Array|Get(acopy) _outactors)))

(fn TriggerShrine)

(fn Reset)