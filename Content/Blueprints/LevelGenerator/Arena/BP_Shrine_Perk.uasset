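; BP_Shrine_Perk is an arena shrine that grants the player a random perk when triggered.
; It extends a parent shrine's trigger event, using a Used flag so the reward fires only once.
; On first trigger it asks the GameManager to add the perk, then swaps the trigger aura's particle template to a reaction effect.
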(event EventBeginPlay
  (|CallParentFunction))

(event EventTriggerShrine
  (|CallParentFunction)
  (if (not (Variables|Default|GetUsed))
    (Variables|Default|SetUsed true)
    (Default|AddRandomPerktoPlayer (Variables|Default|GetGameManager))
    (CallFunction|PlayCollectedPS)))

(fn ConstructionScript
  (|CallParentFunction))

(fn PlayCollectedPS
  (Effects|Components|ParticleSystem|SetTemplate (Variables|Default|GetPS_TriggerAura) "/Game/VFX/particles/p_ShrineReact.p_ShrineReact"))