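; BP_ParentFiller is a base actor Blueprint for level generator filler pieces, displaying a configurable static mesh.
; Its construction script calls SetupMesh, which assigns ActorMesh to the StaticMesh component and applies MeshOffset and MeshScale as relative location and scale.
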(fn ConstructionScript
  (CallFunction|SetupMesh))

(fn SetupMesh
  (Components|StaticMesh|SetStaticMesh (Variables|Default|GetStaticMesh) (Variables|Setup|GetActorMesh))
  (Transformation|SetRelativeLocation (Variables|Default|GetStaticMesh) (Variables|Setup|GetMeshOffset) false false)
  (Transformation|SetRelativeScale3D (Variables|Default|GetStaticMesh) (Variables|Setup|GetMeshScale)))