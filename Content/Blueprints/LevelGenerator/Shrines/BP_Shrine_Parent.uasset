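; BP_Shrine_Parent is the base Blueprint for level-generator shrines that react when the player walks into their trigger.
; On BeginPlay it caches the BP_GameManager found in the world.
; Its TriggerRange overlap filters for BP_MainCharacter and calls TriggerShrine, an empty function left for child shrines to implement.
; The construction script moves TriggerRange to a configurable TriggerOffset.
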(event OnComponentBeginOverlap(TriggerRange)
  (params (OverlappedComponent :type Primitive%20Component%20Object%20Reference) (OtherActor :type Actor%20Object%20Reference) (OtherComp :type Primitive%20Component%20Object%20Reference) (OtherBodyIndex :type Integer) (bFromSweep :type Boolean) (SweepResult :type Hit%20Result%20Structure%20%28by%20ref%29))
  (Utilities|Casting|CastToBP_MainCharacter OtherActor)
  (Core|TriggerShrine))

(event EventBeginPlay
  (Core|GetGameManager))

(fn ConstructionScript
  (Transformation|SetRelativeLocation (Variables|Default|GetTriggerRange) (Variables|Core|GetTriggerOffset) false false))

(fn GetGameManager
  (bind _outactors (Actor|GetAllActorsOfClass "/Game/Blueprints/Management/BP_GameManager.BP_GameManager_C"))
  (Variables|Core|SetGameManager (Utilities|Array|Get(acopy) _outactors)))

(fn TriggerShrine)