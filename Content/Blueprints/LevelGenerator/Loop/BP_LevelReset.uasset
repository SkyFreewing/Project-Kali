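; BP_LevelReset loops the level by teleporting the main character to a reset point and restoring the level's state.
; Overlapping the Trigger moves the player's capsule to ResetPoint, then after a short delay resets shrines, spawners and arena through GameManager and restores the Barrier's visibility and blocking collision.
; ResetPoint, positioned by an offset in the construction script, also switches the player's ambience to the level music on overlap.
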(event OnComponentBeginOverlap(Trigger)
  (params (OverlappedComponent :type Primitive%20Component%20Object%20Reference) (OtherActor :type Actor%20Object%20Reference) (OtherComp :type Primitive%20Component%20Object%20Reference) (OtherBodyIndex :type Integer) (bFromSweep :type Boolean) (SweepResult :type Hit%20Result%20Structure%20%28by%20ref%29))
  (bind _asbp_main_character (Utilities|Casting|CastToBP_MainCharacter OtherActor))
  (CallFunction|TeleportPlayer _asbp_main_character)
  (Utilities|FlowControl|Delay 0.2)
  (CallFunction|ResettheGame))

(event OnComponentBeginOverlap(ResetPoint)
  (params (OverlappedComponent :type Primitive%20Component%20Object%20Reference) (OtherActor :type Actor%20Object%20Reference) (OtherComp :type Primitive%20Component%20Object%20Reference) (OtherBodyIndex :type Integer) (bFromSweep :type Boolean) (SweepResult :type Hit%20Result%20Structure%20%28by%20ref%29))
  (bind _asbp_main_character (Utilities|Casting|CastToBP_MainCharacter OtherActor))
  (Default|UpdateAmbience (Variables|/Game/Blueprints/Characters/MainCharacter/BP_MainCharacter.BP_MainCharacter_C|GetSound%20Manager _asbp_main_character) "/Game/Blueprints/Sound/Music/LevelMusic_mixdown.LevelMusic_mixdown"))

(fn ConstructionScript
  (Transformation|SetRelativeLocation (Variables|Default|GetResetPoint) (Variables|Reset|GetResetOffset) false false))

(fn TeleportPlayer
  (params (Player :type BP%20Main%20Character%20Object%20Reference))
  (Transformation|SetWorldLocation (Variables|/Script/Engine.Character|GetCapsuleComponent Player) (Transformation|GetWorldLocation (Variables|Default|GetResetPoint)) false true))

(fn ResettheGame
  (bind _gamemanager (Variables|Reset|GetGameManager))
  (bind _barrier (Variables|Reset|GetBarrier))
  (Default|ShrinesReset _gamemanager)
  (Default|SpawnersReset _gamemanager)
  (Default|ArenaReset _gamemanager)
  (Rendering|SetVisibility (Variables|/Script/Engine.Actor|GetRootComponent _barrier) true true)
  (Collision|SetCollisionResponsetoChannel (Variables|/Game/Blueprints/LevelGenerator/Arena/BP_Barrier.BP_Barrier_C|GetCube _barrier) "ECC_GameTraceChannel2" "ECR_Block"))