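; Central sound manager that registers with the main character and plays music, Kali's movement and attack sounds, and enemy combat audio.
; It starts level-based ambient music, which can be swapped or replaced by an arena-cleanse track.
; Counters cap and stagger enemy hit and attack sounds and are drained on Tick, alongside a list of growling enemies.
; Tick also prints the current ambient track's name for debugging.
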(event Custom|DelayedPlayHit
  (params (Sound :type Sound%20Base%20Object%20Reference) (Location :type Vector) (Contains? :type Boolean) (Enemy :type BP%20Enemy%20Parent%20Object%20Reference) (SoundSlash :type Sound%20Base%20Object%20Reference))
  (bind _enemygethitsounds (Variables|Default|GetEnemyGetHitSounds))
  ;[1 1 1] EnemyGetHitDelayed
  (Utilities|FlowControl|Delay 0.1)
  (if Contains?
    _
    (else
      (Audio|PlaySoundatLocation Sound Location "0, 0, 0" (* _enemygethitsounds 0.1) 1.0 0.0 "/Game/Blueprints/Sound/EnemySounds.EnemySounds" 0 0)
      (Utilities|Array|Add (Variables|Counter|GetEnemiesGrowling) Enemy)))
  (Audio|PlaySoundatLocation SoundSlash Location "0, 0, 0" _enemygethitsounds 1.0 0.0 0 0 0))

(event Custom|PlaySoundDelayed
  (params (Sound :type Sound%20Base%20Object%20Reference) (Sound2 :type Sound%20Base%20Object%20Reference) (Location :type Vector) (Volume :type Float%20%28single-precision%29))
  ;[1 1 1] SoundsDelayed
  (Utilities|FlowControl|Delay 0.2)
  (Audio|PlaySoundatLocation Sound Location "0, 0, 0" Volume 1.0 0.0 "/Game/Blueprints/Sound/EnemySounds.EnemySounds" 0 0)
  (Audio|PlaySoundatLocation Sound2 Location "0, 0, 0" Volume 1.0 0.0 "/Game/Blueprints/Sound/EnemySounds.EnemySounds" 0 0))

(event EventBeginPlay
  ;[1 1 1] Construct
  (Background|StartAmbience)
  (bind _asbp_main_character (Utilities|Casting|CastToBP_MainCharacter (Game|GetPlayerCharacter 0)))
  (Default|RegisterSoundManager _asbp_main_character self))

(event EventTick
  (params (DeltaSeconds :type Float%20%28single-precision%29))
  (bind _ambient (Variables|Default|GetAmbient))
  (Utilities|IsValid _ambient
    (:Is%20Valid
      ;[1 1 1] Tick
      (Development|PrintString (Utilities|GetDisplayName (Variables|/Script/Engine.AudioComponent|GetSound _ambient)) true true "(R=0.000000,G=0.660000,B=1.000000,A=1.000000)" 0.0))
    (:Is%20Not%20Valid
      _))
  (Utilities|FlowControl|Delay 0.2)
  (if (!= (Variables|Counter|GetEnemiesGettingHit) 0)
    (Utilities|FlowControl|Delay 0.2)
    (Math|Integer|DecrementInt (Variables|Counter|GetEnemiesGettingHit)
      (:%20%20
        (Utilities|Array|RemoveIndex (Variables|Counter|GetEnemiesGrowling)))))
  (if (!= (Variables|Counter|GetEnemiesAttacking) 0)
    (Math|Integer|DecrementInt (Variables|Counter|GetEnemiesAttacking))))

(fn ConstructionScript)

(fn StartAmbience
  (bind _returnvalue (Game|GetCurrentLevelName true))
  (switch name (Utilities|String|StringToName _returnvalue)
    (:Default
      (LocalVariables|SetAmbientStart "/Game/Blueprints/Sound/Music/AfterCleanse_mixdown.AfterCleanse_mixdown" :!label _label))
    (:BlockoutTimo
      (LocalVariables|SetAmbientStart "/Game/Blueprints/Sound/Music/LevelMusic_mixdown.LevelMusic_mixdown"))
    (:MainMenu
      (goto _label)))
  (bind _returnvalue_2 (Audio|CreateSound2D (LocalVariables|GetAmbientStart) (Variables|Default|GetAmbientMusicVolume) 1.0 0.0 0))
  (bind _output_get (Variables|Default|SetAmbient _returnvalue_2))
  (Audio|Components|Audio|Play _output_get 0.0))

(fn AddHitSound
  (params (Sound :type Sound%20Base%20Object%20Reference) (Location :type Vector) (Owner :type BP%20Enemy%20Parent%20Object%20Reference) (SoundImpact :type Sound%20Base%20Object%20Reference))
  (bind _enemiesgettinghit (Variables|Counter|GetEnemiesGettingHit))
  (bind _enemygethitsounds (Variables|Default|GetEnemyGetHitSounds))
  (if (<= _enemiesgettinghit 4)
    (Math|Integer|IncrementInt _enemiesgettinghit
      (:%20%20
        (if (>= _enemiesgettinghit 1)
          (CallFunction|DelayedPlayHit Sound Location false 0 SoundImpact)
          (else
            (if (Utilities|Array|ContainsItem (Variables|Counter|GetEnemiesGrowling) Owner)
              _
              (else
                (Audio|PlaySoundatLocation Sound Location "0, 0, 0" (* _enemygethitsounds 0.2) 1.0 0.0 "/Game/Blueprints/Sound/EnemySounds.EnemySounds" 0 0)
                (Utilities|Array|Add (Variables|Counter|GetEnemiesGrowling) Owner)))
            (Audio|PlaySoundatLocation SoundImpact Location "0, 0, 0" _enemygethitsounds 1.0 0.0 0 0 0)))))))

(fn KaliFootsteps
  (params (Location :type Vector) (Sound :type Sound%20Base%20Object%20Reference))
  (Audio|PlaySoundatLocation Sound Location "0, 0, 0" (Variables|Default|GetKali_FootstepsSounds) 1.0 0.0 0 0 0))

(fn KaliAttackSounds
  (params (Sound :type Sound%20Base%20Object%20Reference) (Location :type Vector))
  (Audio|PlaySoundatLocation Sound Location "0, 0, 0" (Variables|Volume|GetKaliAttackVolume) 1.0 0.0 0 0 0))

(fn AddAttackSound
  (params (Sound :type Sound%20Base%20Object%20Reference) (Location :type Vector))
  (bind _enemiesattacking (Variables|Counter|GetEnemiesAttacking))
  (bind _enemyattackvolume (Variables|Volume|GetEnemyAttackVolume))
  (bind _enemiesattacking_2 (Variables|Counter|GetEnemiesAttacking))
  (if (<= _enemiesattacking 4)
    (if (>= _enemiesattacking 1)
      (Math|Integer|IncrementInt _enemiesattacking_2
        (:%20%20
          (CallFunction|PlaySoundDelayed Sound 0 Location _enemyattackvolume)))
      (else
        (Math|Integer|IncrementInt _enemiesattacking_2
          (:%20%20
            (Audio|PlaySoundatLocation Sound Location "0, 0, 0" _enemyattackvolume 1.0 0.0 "/Game/Blueprints/Sound/EnemySounds.EnemySounds" 0 0)))))))

(fn UpdateAmbience
  (params (NewAmbience :type Sound%20Base%20Object%20Reference))
  (Utilities|IsValid (Variables|Default|GetAmbient)
    (:Is%20Valid
      (Components|DestroyComponent (Variables|Default|GetAmbient)))
    (:Is%20Not%20Valid
      _))
  (bind _returnvalue (Audio|CreateSound2D NewAmbience (Variables|Default|GetAmbientMusicVolume) 1.0 0.0 0))
  (bind _output_get (Variables|Default|SetAmbient _returnvalue))
  (Audio|Components|Audio|Play _output_get 0.0))

(fn ArenaCleanse
  (params (ArenaCleanse :type Sound%20Base%20Object%20Reference))
  (Components|DestroyComponent (Variables|Default|GetAmbient))
  (bind _returnvalue (Audio|CreateSound2D ArenaCleanse (Variables|Default|GetCleanseArenaVolume) 1.0 0.0 0))
  (Audio|Components|Audio|Play _returnvalue 0.0))

(fn KaliDodgeSound
  (params (Location :type Vector) (Sound :type Sound%20Base%20Object%20Reference))
  (Audio|PlaySoundatLocation Sound Location "0, 0, 0" (Variables|Default|GetKali_DodgeSounds) 1.0 0.0 0 0 0))

(fn KaliSpinSounds
  (params (Sound :type Sound%20Base%20Object%20Reference) (Location :type Vector) (Sound2 :type Sound%20Base%20Object%20Reference))
  (bind _kaliattackvolume (Variables|Volume|GetKaliAttackVolume))
  (Audio|PlaySoundatLocation Sound Location "0, 0, 0" _kaliattackvolume 1.0 0.0 0 0 0)
  (Audio|PlaySoundatLocation Sound2 Location "0, 0, 0" _kaliattackvolume 1.0 0.0 0 0 0))