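; Base enemy character that spawns a sword, runs BT_EnemyAI through blackboard flags and alerts its squad on hearing noise or taking radial damage.
; Tick polls tracked player-sword collider overlaps against the player's hit windows, with brief invulnerability.
; Radial damage types select damage, stun, aggro or knockback.
; Tick also turns the status widget toward the camera and handles dissolve or sinking deaths and distance-based despawning.
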(event OnComponentBeginOverlap(CapsuleComponent)
  (params (OverlappedComponent :type Primitive%20Component%20Object%20Reference) (OtherActor :type Actor%20Object%20Reference) (OtherComp :type Primitive%20Component%20Object%20Reference) (OtherBodyIndex :type Integer) (bFromSweep :type Boolean) (SweepResult :type Hit%20Result%20Structure%20%28by%20ref%29))
  ;[1 1 1] Get Overlapping Object
  (CheckHit|BeginOverlap OtherActor))

(event OnComponentEndOverlap(CapsuleComponent)
  (params (OverlappedComponent :type Primitive%20Component%20Object%20Reference) (OtherActor :type Actor%20Object%20Reference) (OtherComp :type Primitive%20Component%20Object%20Reference) (OtherBodyIndex :type Integer))
  ;[1 1 1] Get Overlapping Object
  (CheckHit|EndOverlap OtherActor))

(event OnHearNoise(PawnSensing)
  (params (Instigator :type Pawn%20Object%20Reference) (Location :type Vector%20%28by%20ref%29 :default "0, 0, 0") (Volume :type Float%20%28single-precision%29))
  ;[0.962 0.1801 1] AI (Spidey Senses)
  (if (not (Variables|Combat|GetIsStunned))
    (Combat|TargetPlayer)
    (if (not (Variables|AI|GetSquadAlerted))
      (AI|AlertSquad))))

(event Custom|Checkdistance
  ;[1 1 1] Check Despawndistance
  (Core|CheckDespawnDistance))

(event Custom|EndStagger
  ;[1 0.269 0.3188] Combat
  ;;[1 1 1] Take Damage
  (Variables|Combat|SetIsStunned false)
  (AI|AlertSquad))

(event Game|Damage|EventRadialDamage
  (params (DamageReceived :type Float%20%28single-precision%29) (DamageType :type Damage%20Type%20Object%20Reference) (Origin :type Vector :default "0, 0, 0") (HitInfo :type Hit%20Result%20Structure%20%28by%20ref%29) (InstigatedBy :type Controller%20Object%20Reference) (DamageCauser :type Actor%20Object%20Reference))
  ;[1 0.269 0.3188] Combat
  ;;[1 1 1] Radial Damage
  (bind _stunned_ (Combat|ProcessDamage DamageReceived DamageType))
  (bind _asbp_main_character (Utilities|Casting|CastToBP_MainCharacter DamageCauser))
  (Default|AbilityHits _asbp_main_character)
  (if _stunned_
    (Utilities|FlowControl|Delay DamageReceived)
    (Variables|Combat|SetIsStunned false)
    (else
      (Utilities|FlowControl|Delay 1.0)))
  (AI|AlertSquad))

(event EventTick
  (params (DeltaSeconds :type Float%20%28single-precision%29))
  ;[0 0 0] Core
  ;;[1 1 1] Tick
  (if (Variables|Combat|GetDying)
    (Combat|Dissolve)
    (if (Variables|Despawning|GetSinking)
      (Variables|Despawning|SetSinking false)
      (Variables|Despawning|SetSinkingStartLocation (Transformation|GetActorLocation))
      (bind _height (Timeline|TimelineSinking Play)
        (:Update
          (Transformation|SetActorLocation (Math|Vector|MakeVector (.x (Variables|Despawning|GetSinkingStartLocation)) (.y (Variables|Despawning|GetSinkingStartLocation)) (+ (.z (Variables|Despawning|GetSinkingStartLocation)) _height)) false false))
        (:Finished
          (Death|DestroyActor :!label _label)))
      (else
        (Utilities|FlowControl|Delay 0.5)
        (Death|DestroyActor)))
    (elif (Variables|Despawning|GetDespawning)
      (Utilities|FlowControl|Delay 1.0)
      (bind _result (Math|Float|DecrementFloat (Variables|Despawning|GetDespawnCountdown))
        (:%20%20
          (if (and (== _result 0.0) (Variables|Despawning|GetDespawning))
            (goto _label))))
      (else
        (UI|DirectUItoPlayer)
        (if (Variables|Combat|GetHitInvul)
          (Utilities|FlowControl|Delay (Variables|Combat|GetInvulTimer))
          (Variables|Combat|SetInvulTimer 0.33)
          (Variables|Combat|SetHitInvul false)
          (if (not (Variables|Despawning|GetDespawning))
            ;[1 0.269 0.3188] Combat
            ;;[1 1 1] Take Damage
            (if (not (and (Math|Boolean|ORBoolean (Variables|Combat|GetColliderTopLeftFilled) (Variables|Combat|GetColliderTopRightFilled) (Variables|Combat|GetColliderBottomRightFilled) (Variables|Combat|GetColliderBottomleftFilled)) (Variables|Combat|GetHitInvul))) :!label _label_2
              (bind _isattacking (Combat|CheckHit))
              (if _isattacking
                (Variables|Combat|SetHitInvul true))))
          (else
            (goto _label_2)))))))

(event EventBeginPlay
  ;[0 0 0] Core
  ;;[1 1 1] Startup
  (bind _aswbp_dummy_enemy_status (Utilities|Casting|CastToWBP_DummyEnemy_Status (UserInterface|GetUserWidgetObject (Variables|Default|GetStatusWidget))))
  (bind _output_get (Variables|UI|SetDummyWidget _aswbp_dummy_enemy_status))
  (SetUp|SetupBehaviour)
  (SetUp|SetupWeapon))

(fn ConstructionScript
  (Core|SetupEnemy)
  (UI|SetupUI))

(fn SetupUI
  (Transformation|SetRelativeLocation (Variables|Default|GetStatusWidget) (Variables|UI|GetStatusUIOffset) false false)
  (Transformation|SetRelativeLocation (Variables|Default|GetFocusWidget) (Variables|UI|GetFocusUIOffset) false false))

(fn AlterHealth
  (params (HealthChange :type Float%20%28single-precision%29))
  (bind _output_get (Variables|Ressources|SetHealth (Math|Float|Clamp(Float) (+ HealthChange (Variables|Ressources|GetHealth)) 0.0 (Variables|Ressources|GetMaxHealth))))
  (bind _asbp_main_character (Utilities|Casting|CastToBP_MainCharacter (Game|GetPlayerCharacter 0)))
  (Default|RaiseCombo _asbp_main_character)
  (if (== _output_get 0.0)
    (Default|AddExp _asbp_main_character (Variables|Combat|GetaddsEXP))
    (Variables|Combat|SetDying true)
    (else
      (Default|UpdateHealth (Variables|UI|GetDummyWidget) (Variables|Ressources|GetHealth)))))

(fn SetupEnemy
  (Variables|Ressources|SetHealth (Variables|Ressources|GetMaxHealth))
  (Setup|Setup))

(fn DirectUItoPlayer
  (Transformation|SetWorldRotation (Variables|Default|GetStatusWidget) (Math|Rotator|FindLookatRotation (Transformation|GetWorldLocation (Variables|Default|GetStatusWidget)) (Camera|GetCameraLocation (Game|GetPlayerCameraManager 0))) false false))

(fn SetupBehaviour
  (bind _self self)
  (AI|RunBehaviorTree (AI|GetAIController _self) "/Game/Blueprints/Characters/EnemyDummy/BT_EnemyAI.BT_EnemyAI")
  (AI|Components|Blackboard|SetValueasBool (AI|GetBlackboard _self) (Utilities|Name|MakeLiteralName "Idle") true))

(fn CheckHit
  (bind _soundmanager (Variables|Management|GetSoundManager))
  (bind _asbp_main_character (Utilities|Casting|CastToBP_MainCharacter (Game|GetPlayerCharacter 0)))
  (bind _canattack (Combat|CheckSword _asbp_main_character))
  (if _canattack
    (Combat|ProcessStun)
    (Default|ApplyRage _asbp_main_character (/ (Math|Conversions|ToFloat(Integer) (Variables|/Game/Blueprints/Characters/MainCharacter/BP_MainCharacter.BP_MainCharacter_C|GetBasicAttackDMG _asbp_main_character)) -2e+01))
    (Combat|Knockback 1e+01)
    (UI|AlterHealth (Math|Conversions|ToFloat(Integer) (Variables|/Game/Blueprints/Characters/MainCharacter/BP_MainCharacter.BP_MainCharacter_C|GetBasicAttackDMG _asbp_main_character)))
    (if (Utilities|IsValid _soundmanager)
      (Default|EnemyGetsHit _soundmanager self)))
  (return _canattack))

(fn SetupWeapon
  (bind _returnvalue (Game|SpawnActorfromClass "/Game/Blueprints/Combat/BP_EnemySword_V1.BP_EnemySword_V1_C" (Transformation|GetSocketTransform (Variables|Character|GetMesh) "WeaponSlot" "RTS_ParentBoneSpace") "Undefined" 0 0))
  (Variables|/Game/Blueprints/Combat/BP_EnemySword_V1.BP_EnemySword_V1_C|SetWielder _returnvalue self)
  (bind _output_get (Variables|Ressources|SetWeapon _returnvalue))
  (Transformation|AttachComponentToComponent _output_get (Variables|Character|GetMesh) "WeaponSlot" "SnapToTarget" "SnapToTarget" "KeepRelative" true))

(fn AiAttack
  (if (not (Variables|Combat|GetIsStunned))
    (Variables|Combat|SetAttacking true)
    (AI|Components|Blackboard|SetValueasBool (AI|GetBlackboard self) (Utilities|Name|MakeLiteralName "Attacking") true)))

(fn ProcessDamage
  (params (Damage :type Float%20%28single-precision%29) (DamageType :type Damage%20Type%20Object%20Reference))
  (Utilities|Casting|CastToDTBP_DamageTypeCircl DamageType
    (:then
      (UI|AlterHealth Damage)
      (return false))
    (:CastFailed
      (Utilities|Casting|CastToDTBP_DamageTypeStun DamageType
        (:then
          (Combat|ProcessStun)
          (return true))
        (:CastFailed
          (Utilities|Casting|CastToDTBP_DamageTypeAggro DamageType
            (:then
              (Combat|TargetPlayer)
              (return false))
            (:CastFailed
              (Utilities|Casting|CastToDTBP_DamageTypeKnockBack DamageType)
              (Combat|Knockback 15.0)
              (return false))))))))

(fn ProcessStun
  (Variables|Combat|SetIsStunned true)
  (AI|Components|Blackboard|SetValueasBool (AI|GetBlackboard self) (Utilities|Name|MakeLiteralName "Idle") false)
  (AI|Components|Blackboard|SetValueasBool (AI|GetBlackboard self) (Utilities|Name|MakeLiteralName "AttackIntent") false)
  (AI|Components|Blackboard|SetValueasBool (AI|GetBlackboard self) (Utilities|Name|MakeLiteralName "Stunned") true))

(fn TargetPlayer
  (if (not (Variables|Combat|GetIsStunned))
    (Variables|Despawning|SetDespawning false)
    (AI|Components|Blackboard|SetValueasBool (AI|GetBlackboard 0) (Utilities|Name|MakeLiteralName "Idle") false)
    (AI|Components|Blackboard|SetValueasBool (AI|GetBlackboard 0) (Utilities|Name|MakeLiteralName "AttackIntent") true)
    (AI|Components|Blackboard|SetValueasBool (AI|GetBlackboard 0) (Utilities|Name|MakeLiteralName "Stunned") false)))

(fn Knockback
  (params (Scale :type Float%20%28single-precision%29))
  (Variables|Combat|SetIsStunned true))

(fn LowerFriction
  (bind _charactermovement (Variables|Character|GetCharacterMovement))
  (Variables|/Script/Engine.CharacterMovementComponent|SetBrakingFriction _charactermovement 0.0)
  (Variables|/Script/Engine.CharacterMovementComponent|SetBrakingDecelerationWalking _charactermovement 0.0)
  (Variables|/Script/Engine.CharacterMovementComponent|SetMaxWalkSpeed _charactermovement 2e+03))

(fn RaiseFriction
  (bind _charactermovement (Variables|Character|GetCharacterMovement))
  (Variables|/Script/Engine.CharacterMovementComponent|SetBrakingFriction _charactermovement 1.0)
  (Variables|/Script/Engine.CharacterMovementComponent|SetBrakingDecelerationWalking _charactermovement 2048.0)
  (Variables|/Script/Engine.CharacterMovementComponent|SetMaxWalkSpeed _charactermovement 4e+02))

(fn ProcessCharge
  (if (not (Variables|Combat|GetHitInvul))
    (bind _asbp_main_character (Utilities|Casting|CastToBP_MainCharacter (Game|GetPlayerCharacter 0)))
    (Default|AbilityHits _asbp_main_character)
    (UI|AlterHealth (Variables|/Game/Blueprints/Characters/MainCharacter/BP_MainCharacter.BP_MainCharacter_C|GetChargeDamage _asbp_main_character))
    (Combat|Knockback 4e+01)
    (Variables|Combat|SetHitInvul true)))

(fn ToggleTargetMarker
  (params (Visibility :type Boolean))
  (Rendering|SetRenderCustomDepth (Variables|Character|GetMesh) Visibility))

(fn BeginOverlap
  (params (Actor :type Actor%20Object%20Reference))
  (Utilities|Casting|CastToBP_KaliSword_LeftTop Actor
    (:then
      (Variables|Combat|SetColliderTopLeft Actor)
      (Variables|Combat|SetColliderTopLeftFilled true))
    (:CastFailed
      (Utilities|Casting|CastToBP_KaliSword_LeftBottom Actor
        (:then
          (Variables|Combat|SetColliderBottomleft Actor)
          (Variables|Combat|SetColliderBottomleftFilled true))
        (:CastFailed
          (Utilities|Casting|CastToBP_KaliSword_RightBottom Actor
            (:then
              (Variables|Combat|SetColliderBottomRight Actor)
              (Variables|Combat|SetColliderBottomRightFilled true))
            (:CastFailed
              (Utilities|Casting|CastToBP_KaliSword_RightTop Actor)
              (Variables|Combat|SetColliderTopRight Actor)
              (Variables|Combat|SetColliderTopRightFilled true))))))))

(fn CheckSword
  (params (Main%20Character :type BP%20Main%20Character%20Object%20Reference))
  (return (or (and (Variables|/Game/Blueprints/Characters/MainCharacter/BP_MainCharacter.BP_MainCharacter_C|GetCanHitLeft Main%20Character) (or (Variables|Combat|GetColliderTopLeftFilled) (Variables|Combat|GetColliderBottomleftFilled))) (and (Variables|/Game/Blueprints/Characters/MainCharacter/BP_MainCharacter.BP_MainCharacter_C|GetCanHitRight Main%20Character) (or (Variables|Combat|GetColliderTopRightFilled) (Variables|Combat|GetColliderBottomRightFilled))))))

(fn EndOverlap
  (params (Actor :type Actor%20Object%20Reference))
  (if (== Actor (Variables|Combat|GetColliderTopLeft))
    (Variables|Combat|SetColliderTopLeft 0)
    (Variables|Combat|SetColliderTopLeftFilled false)
    (elif (== Actor (Variables|Combat|GetColliderTopRight))
      (Variables|Combat|SetColliderTopRight 0)
      (Variables|Combat|SetColliderTopRightFilled false)
      (elif (== Actor (Variables|Combat|GetColliderBottomRight))
        (Variables|Combat|SetColliderBottomRight 0)
        (Variables|Combat|SetColliderBottomRightFilled false)
        (elif (== Actor (Variables|Combat|GetColliderBottomleft))
          (Variables|Combat|SetColliderBottomleft 0)
          (Variables|Combat|SetColliderBottomleftFilled false))))))

(fn CheckDespawnDistance
  (if (>= (Transformation|GetDistanceTo self (Game|GetPlayerCharacter 0)) (Variables|Despawning|GetDespawnDistance))
    (if (not (Variables|Despawning|GetDespawning))
      (Variables|Despawning|SetDespawning true)
      (Variables|Despawning|SetDespawnCountdown 2.0))
    (elif (Variables|Despawning|GetDespawning)
      (Variables|Despawning|SetDespawning false))))

(fn AlertSquad
  (if (not (Variables|Combat|GetIsStunned))
    (Variables|AI|SetSquadAlerted true)
    (for _array_element (Variables|AI|GetSquad)
      (Utilities|IsValid _array_element
        (:Is%20Valid
          (Combat|TargetPlayer _array_element)
          (Variables|BP_Enemy_Parent_C|SetSquadAlerted _array_element true))))))

(fn SquadWaypoint
  (params (Waypoint :type Vector))
  (Variables|AI|SetSquadhasWaypoint true)
  (for _array_element (Variables|AI|GetSquad)
    (Utilities|IsValid _array_element
      (:Is%20Valid
        (Variables|BP_Enemy_Parent_C|SetNextWaypoint _array_element Waypoint)
        (Variables|AI|SetSquadhasWaypoint _array_element true)))))

(fn DestroyActor
  (Utilities|Array|RemoveIndex (Variables|AI|GetSquad) (Utilities|Array|FindItem (Variables|AI|GetSquad) self))
  (for _array_element (Variables|AI|GetSquad)
    (Variables|BP_Enemy_Parent_C|SetSquad _array_element (Variables|AI|GetSquad)))
  (Actor|DestroyActor (Variables|Ressources|GetWeapon))
  (Actor|DestroyActor))

(fn Setup
  (bind _returnvalue (Class|LayersBlueprintLibrary|GetActors (Utilities|Struct|MakeActorLayer (Utilities|Name|MakeLiteralName "Management"))))
  (bind _asbp_game_manager (Utilities|Casting|CastToBP_GameManager (Utilities|Array|Get(acopy) _returnvalue))
    (:then
      (Variables|Management|SetGameManager _asbp_game_manager))
    (:CastFailed
      _))
  (bind _returnvalue_2 (Class|LayersBlueprintLibrary|GetActors (Utilities|Struct|MakeActorLayer (Utilities|Name|MakeLiteralName "Sound"))))
  (bind _asbp_sound_manager (Utilities|Casting|CastToBP_SoundManager (Utilities|Array|Get(acopy) _returnvalue_2)))
  (Variables|Management|SetSoundManager _asbp_sound_manager))

(fn Dissolve
  (bind _mesh (Variables|Character|GetMesh))
  (if (Variables|Despawning|GetDissolving)
    (Variables|Despawning|SetDissolving false)
    (bind _returnvalue (Rendering|Material|CreateDynamicMaterialInstance _mesh 0 (Rendering|Material|GetMaterial _mesh 0) "None" :!class /Script/Engine.PrimitiveComponent))
    (Rendering|Material|SetScalarParameterValue _returnvalue "Dissolve Amount" (Math|Interpolation|FInterpTo 0.0 1.0 (Utilities|Time|GetWorldDeltaSeconds) 5.0) :!class /Script/Engine.MaterialInstanceDynamic)))

(fn DeathbyWater
  (AI|Components|Blackboard|SetValueasBool (AI|GetBlackboard self) (Utilities|Name|MakeLiteralName "Idle") false)
  (AI|Components|Blackboard|SetValueasBool (AI|GetBlackboard self) (Utilities|Name|MakeLiteralName "AttackIntent") false)
  (AI|Components|Blackboard|SetValueasBool (AI|GetBlackboard self) (Utilities|Name|MakeLiteralName "Stunned") true)
  (Variables|Despawning|SetSinking true)
  (Variables|Combat|SetDying true)
  (bind _asbp_main_character (Utilities|Casting|CastToBP_MainCharacter (Game|GetPlayerCharacter 0)))
  (Default|AddExp _asbp_main_character (Variables|Combat|GetaddsEXP)))