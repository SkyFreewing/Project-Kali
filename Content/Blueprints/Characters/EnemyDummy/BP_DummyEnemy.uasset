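; Squad-based melee enemy that spawns a sword, runs BT_EnemyAI, attacks with a timeline-driven rotation and shows a camera-facing status widget.
; Tick polls overlaps with the player's four sword colliders, while damage-type classes route radial hits to damage, stun, aggro or knockback.
; Sightings and hits alert the squad through blackboard flags.
; Health loss raises player combo and death grants EXP; distant enemies despawn after a countdown.
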(event OnComponentBeginOverlap(CapsuleComponent)
  (params (OverlappedComponent :type Primitive%20Component%20Object%20Reference) (OtherActor :type Actor%20Object%20Reference) (OtherComp :type Primitive%20Component%20Object%20Reference) (OtherBodyIndex :type Integer) (bFromSweep :type Boolean) (SweepResult :type Hit%20Result%20Structure%20%28by%20ref%29))
  ;[1 1 1] Get Overlapping Object
  (CheckHit|BeginOverlap OtherActor))

(event OnSeePawn(PawnSensing)
  (params (Pawn :type Pawn%20Object%20Reference))
  ;[0.962 0.1801 1] AI
  (Combat|TargetPlayer)
  (if (not (Variables|AI|GetSquadAlerted))
    (AI|AlertSquad)))

(event OnComponentEndOverlap(CapsuleComponent)
  (params (OverlappedComponent :type Primitive%20Component%20Object%20Reference) (OtherActor :type Actor%20Object%20Reference) (OtherComp :type Primitive%20Component%20Object%20Reference) (OtherBodyIndex :type Integer))
  ;[1 1 1] Get Overlapping Object
  (CheckHit|EndOverlap OtherActor))

(event Custom|AIAttacking
  ;[1 0.269 0.3188] Combat
  ;;[1 1 1] Attack
  (Variables|Combat|SetStartrotation (.Yaw (Math|Rotator|BreakRotator (Pawn|GetControlRotation :!class /Script/Engine.Pawn))))
  (bind _rotation (Timeline|Timeline_0 PlayFromStart)
    (:Update
      (Transformation|SetActorRotation (Math|Rotator|MakeRotator 0.0 0.0 (+ _rotation (Variables|Combat|GetStartrotation)))))
    (:Finished
      (Variables|Combat|SetIsAttacking false))))

(event Custom|Checkdistance
  ;[1 1 1] Räumen sie ihren Kram auf, Sir
  (Core|CheckDespawnDistance))

(event Game|Damage|EventRadialDamage
  (params (DamageReceived :type Float%20%28single-precision%29) (DamageType :type Damage%20Type%20Object%20Reference) (Origin :type Vector :default "0, 0, 0") (HitInfo :type Hit%20Result%20Structure%20%28by%20ref%29) (InstigatedBy :type Controller%20Object%20Reference) (DamageCauser :type Actor%20Object%20Reference))
  (bind _stunned_ (Combat|ProcessDamage DamageReceived DamageType))
  (bind _asbp_main_character (Utilities|Casting|CastToBP_MainCharacter DamageCauser))
  (Default|AbilityHits _asbp_main_character)
  (if _stunned_
    (Utilities|FlowControl|Delay DamageReceived)
    (else
      (Utilities|FlowControl|Delay 1.0)))
  (AI|AlertSquad))

(event EventTick
  (params (DeltaSeconds :type Float%20%28single-precision%29))
  ;[0 0 0] Core
  ;;[1 1 1] Tick
  (if (Variables|Despawning|GetDespawning)
    (Utilities|FlowControl|Delay 1.0)
    (bind _result (Math|Float|DecrementFloat (Variables|Despawning|GetDespawnCountdown))
      (:%20%20
        (if (and (== _result 0.0) (Variables|Despawning|GetDespawning))
          (Death|DestroyActor))))
    (else
      (UI|DirectUItoPlayer)
      (if (Variables|Combat|GetHitInvul)
        (Utilities|FlowControl|Delay (Variables|Combat|GetInvulTimer))
        (Variables|Combat|SetInvulTimer 0.33)
        (Variables|Combat|SetHitInvul false)
        (if (not (Variables|Despawning|GetDespawning))
          ;[1 0.269 0.3188] Combat
          ;;[1 1 1] Take Damage
          (if (not (and (Math|Boolean|ORBoolean (Variables|Combat|GetColliderTopLeftFilled) (Variables|Combat|GetColliderTopRightFilled) (Variables|Combat|GetColliderBottomRightFilled) (Variables|Combat|GetColliderBottomleftFilled)) (Variables|Combat|GetHitInvul))) :!label _label
            (bind _isattacking (Combat|CheckHit))
            (if _isattacking
              (Variables|Combat|SetHitInvul true)
              (Utilities|FlowControl|Delay (Variables|Combat|GetHitStaggerTime))
              (AI|AlertSquad))))
        (else
          (goto _label))))))

(event EventBeginPlay
  ;[0 0 0] Core
  ;;[1 1 1] Startup
  (bind _aswbp_dummy_enemy_status (Utilities|Casting|CastToWBP_DummyEnemy_Status (UserInterface|GetUserWidgetObject (Variables|Default|GetStatusWidget))))
  (Variables|UI|SetDummyWidget _aswbp_dummy_enemy_status)
  (Utilities|FlowControl|Delay 0.75)
  (SetUp|SetupBehaviour)
  (SetUp|SetupWeapon))

(fn ConstructionScript
  (Core|SetupEnemy)
  (UI|SetupUI))

(fn SetupUI
  (Transformation|SetRelativeLocation (Variables|Default|GetStatusWidget) (Variables|UI|GetStatusUIOffset) false false)
  (Transformation|SetRelativeLocation (Variables|Default|GetFocusWidget) (Variables|UI|GetFocusUIOffset) false false))

(fn AlterHealth
  (params (HealthChange :type Float%20%28single-precision%29))
  (bind _output_get (Variables|Ressources|SetHealth (Math|Float|Clamp(Float) (+ HealthChange (Variables|Ressources|GetHealth)) 0.0 (Variables|Ressources|GetMaxHealth))))
  (bind _asbp_main_character (Utilities|Casting|CastToBP_MainCharacter (Game|GetPlayerCharacter 0)))
  (Default|RaiseCombo _asbp_main_character)
  (if (== _output_get 0.0)
    (Default|AddExp _asbp_main_character (Variables|Combat|GetaddsEXP))
    (Death|DestroyActor)
    (else
      (Default|UpdateHealth (Variables|UI|GetDummyWidget) (Variables|Ressources|GetHealth)))))

(fn SetupEnemy
  (Variables|Ressources|SetHealth (Variables|Ressources|GetMaxHealth)))

(fn DirectUItoPlayer
  (Transformation|SetWorldRotation (Variables|Default|GetStatusWidget) (Math|Rotator|FindLookatRotation (Transformation|GetWorldLocation (Variables|Default|GetStatusWidget)) (Camera|GetCameraLocation (Game|GetPlayerCameraManager 0))) false false))

(fn SetupBehaviour
  (bind _self self)
  (AI|RunBehaviorTree (AI|GetAIController _self) "/Game/Blueprints/Characters/EnemyDummy/BT_EnemyAI.BT_EnemyAI")
  (AI|Components|Blackboard|SetValueasBool (AI|GetBlackboard _self) (Utilities|Name|MakeLiteralName "Idle") true))

(fn CheckHit
  (bind _asbp_main_character (Utilities|Casting|CastToBP_MainCharacter (Game|GetPlayerCharacter 0)))
  (bind _canattack (Combat|CheckSword _asbp_main_character))
  (if _canattack
    (Combat|ProcessStun)
    (Default|ApplyRage _asbp_main_character (/ (Math|Conversions|ToFloat(Integer) (Variables|/Game/Blueprints/Characters/MainCharacter/BP_MainCharacter.BP_MainCharacter_C|GetBasicAttackDMG _asbp_main_character)) -2e+01))
    (Combat|Knockback 1e+01)
    (UI|AlterHealth (Math|Conversions|ToFloat(Integer) (Variables|/Game/Blueprints/Characters/MainCharacter/BP_MainCharacter.BP_MainCharacter_C|GetBasicAttackDMG _asbp_main_character))))
  (return _canattack))

(fn SetupWeapon
  (bind _returnvalue (Game|SpawnActorfromClass "/Game/Blueprints/Combat/BP_EnemySword_V1.BP_EnemySword_V1_C" (Transformation|GetSocketTransform (Variables|Character|GetMesh) "WeaponSlot" "RTS_ParentBoneSpace") "Undefined" 0 0))
  (Variables|/Game/Blueprints/Combat/BP_EnemySword_V1.BP_EnemySword_V1_C|SetWielder _returnvalue self)
  (bind _output_get (Variables|Ressources|SetWeapon _returnvalue))
  (Transformation|AttachComponentToComponent _output_get (Variables|Character|GetMesh) "WeaponSlot" "KeepRelative" "KeepRelative" "KeepRelative" true))

(fn AiAttack
  (if (not (Variables|Combat|GetIsAttacking))
    (Variables|Combat|SetIsAttacking true)
    (CallFunction|AIAttacking)))

(fn ProcessDamage
  (params (Damage :type Float%20%28single-precision%29) (DamageType :type Damage%20Type%20Object%20Reference))
  (Utilities|Casting|CastToDTBP_DamageTypeCircl DamageType
    (:then
      (UI|AlterHealth Damage)
      (return false))
    (:CastFailed
      (Utilities|Casting|CastToDTBP_DamageTypeStun DamageType
        (:then
          (Combat|ProcessStun)
          (return true))
        (:CastFailed
          (Utilities|Casting|CastToDTBP_DamageTypeAggro DamageType
            (:then
              (Combat|TargetPlayer)
              (return false))
            (:CastFailed
              (Utilities|Casting|CastToDTBP_DamageTypeKnockBack DamageType)
              (Combat|Knockback 1e+01)
              (return false))))))))

(fn ProcessStun
  (AI|Components|Blackboard|SetValueasBool (AI|GetBlackboard self) (Utilities|Name|MakeLiteralName "Idle") false)
  (AI|Components|Blackboard|SetValueasBool (AI|GetBlackboard self) (Utilities|Name|MakeLiteralName "AttackIntent") false)
  (AI|Components|Blackboard|SetValueasBool (AI|GetBlackboard self) (Utilities|Name|MakeLiteralName "Stunned") true))

(fn TargetPlayer
  (Variables|Despawning|SetDespawning false)
  (AI|Components|Blackboard|SetValueasBool (AI|GetBlackboard self) (Utilities|Name|MakeLiteralName "Idle") false)
  (AI|Components|Blackboard|SetValueasBool (AI|GetBlackboard self) (Utilities|Name|MakeLiteralName "AttackIntent") true)
  (AI|Components|Blackboard|SetValueasBool (AI|GetBlackboard self) (Utilities|Name|MakeLiteralName "Stunned") false))

(fn Knockback
  (params (Scale :type Float%20%28single-precision%29))
  (bind _asbp_main_character (Utilities|Casting|CastToBP_MainCharacter (Game|GetPlayerCharacter 0)))
  (Character|LaunchCharacter (* (Math|Vector|MakeVector (.X (Math|Vector|BreakVector (- (Transformation|GetActorLocation) (Transformation|GetActorLocation _asbp_main_character)))) (.Y (Math|Vector|BreakVector (- (Transformation|GetActorLocation) (Transformation|GetActorLocation _asbp_main_character)))) 0.0) Scale) false false))

(fn LowerFriction
  (bind _charactermovement (Variables|Character|GetCharacterMovement))
  (Variables|/Script/Engine.CharacterMovementComponent|SetBrakingFriction _charactermovement 0.0)
  (Variables|/Script/Engine.CharacterMovementComponent|SetBrakingDecelerationWalking _charactermovement 0.0)
  (Variables|/Script/Engine.CharacterMovementComponent|SetMaxWalkSpeed _charactermovement 2e+03))

(fn RaiseFriction
  (bind _charactermovement (Variables|Character|GetCharacterMovement))
  (Variables|/Script/Engine.CharacterMovementComponent|SetBrakingFriction _charactermovement 1.0)
  (Variables|/Script/Engine.CharacterMovementComponent|SetBrakingDecelerationWalking _charactermovement 2048.0)
  (Variables|/Script/Engine.CharacterMovementComponent|SetMaxWalkSpeed _charactermovement 4e+02))

(fn ProcessCharge
  (if (not (Variables|Combat|GetHitInvul))
    (bind _asbp_main_character (Utilities|Casting|CastToBP_MainCharacter (Game|GetPlayerCharacter 0)))
    (Default|AbilityHits _asbp_main_character)
    (Development|PrintString "Charge Damage")
    (UI|AlterHealth (Variables|/Game/Blueprints/Characters/MainCharacter/BP_MainCharacter.BP_MainCharacter_C|GetChargeDamage _asbp_main_character))
    (if (Variables|/Game/Blueprints/Characters/MainCharacter/BP_MainCharacter.BP_MainCharacter_C|GetStopsOnFirst _asbp_main_character)
      (Variables|Combat|SetHitInvul true)
      (Default|StopCharge _asbp_main_character)
      (else
        (Variables|Combat|SetInvulTimer 0.6)
        (Variables|Combat|SetHitInvul true)
        (Development|PrintString "BIG Oooof")))))

(fn ToggleTargetMarker
  (params (Visibility :type Boolean))
  (Rendering|SetRenderCustomDepth (Variables|Character|GetMesh) Visibility))

(fn BeginOverlap
  (params (Actor :type Actor%20Object%20Reference))
  (Utilities|Casting|CastToBP_KaliSword_LeftTop Actor
    (:then
      (Variables|Combat|SetColliderTopLeft Actor)
      (Variables|Combat|SetColliderTopLeftFilled true))
    (:CastFailed
      (Utilities|Casting|CastToBP_KaliSword_LeftBottom Actor
        (:then
          (Variables|Combat|SetColliderBottomleft Actor)
          (Variables|Combat|SetColliderBottomleftFilled true))
        (:CastFailed
          (Utilities|Casting|CastToBP_KaliSword_RightBottom Actor
            (:then
              (Variables|Combat|SetColliderBottomRight Actor)
              (Variables|Combat|SetColliderBottomRightFilled true))
            (:CastFailed
              (Utilities|Casting|CastToBP_KaliSword_RightTop Actor)
              (Variables|Combat|SetColliderTopRight Actor)
              (Variables|Combat|SetColliderTopRightFilled true))))))))

(fn CheckSword
  (params (Main%20Character :type BP%20Main%20Character%20Object%20Reference))
  (return (or (and (Variables|/Game/Blueprints/Characters/MainCharacter/BP_MainCharacter.BP_MainCharacter_C|GetCanHitLeft Main%20Character) (or (Variables|Combat|GetColliderTopLeftFilled) (Variables|Combat|GetColliderBottomleftFilled))) (and (Variables|/Game/Blueprints/Characters/MainCharacter/BP_MainCharacter.BP_MainCharacter_C|GetCanHitRight Main%20Character) (or (Variables|Combat|GetColliderTopRightFilled) (Variables|Combat|GetColliderBottomRightFilled))))))

(fn EndOverlap
  (params (Actor :type Actor%20Object%20Reference))
  (if (== Actor (Variables|Combat|GetColliderTopLeft))
    (Variables|Combat|SetColliderTopLeft 0)
    (Variables|Combat|SetColliderTopLeftFilled false)
    (elif (== Actor (Variables|Combat|GetColliderTopRight))
      (Variables|Combat|SetColliderTopRight 0)
      (Variables|Combat|SetColliderTopRightFilled false)
      (elif (== Actor (Variables|Combat|GetColliderBottomRight))
        (Variables|Combat|SetColliderBottomRight 0)
        (Variables|Combat|SetColliderBottomRightFilled false)
        (elif (== Actor (Variables|Combat|GetColliderBottomleft))
          (Variables|Combat|SetColliderBottomleft 0)
          (Variables|Combat|SetColliderBottomleftFilled false))))))

(fn CheckDespawnDistance
  (if (>= (Transformation|GetDistanceTo self (Game|GetPlayerCharacter 0)) (Variables|Despawning|GetDespawnDistance))
    (if (not (Variables|Despawning|GetDespawning))
      (Variables|Despawning|SetDespawning true)
      (Variables|Despawning|SetDespawnCountdown 2.0))
    (elif (Variables|Despawning|GetDespawning)
      (Variables|Despawning|SetDespawning false))))

(fn AlertSquad
  (Variables|AI|SetSquadAlerted true)
  (for _array_element (Variables|AI|GetSquad)
    (Utilities|IsValid _array_element
      (:Is%20Valid
        (Combat|TargetPlayer _array_element)
        (Variables|BP_DummyEnemy_C|SetSquadAlerted _array_element true)))))

(fn SquadWaypoint
  (params (Waypoint :type Vector))
  (Variables|AI|SetSquadhasWaypoint true)
  (for _array_element (Variables|AI|GetSquad)
    (Utilities|IsValid _array_element
      (:Is%20Valid
        (Variables|BP_DummyEnemy_C|SetNextWaypoint _array_element Waypoint)
        (Variables|AI|SetSquadhasWaypoint _array_element true)))))

(fn DestroyActor
  (Utilities|Array|RemoveIndex (Variables|AI|GetSquad) (Utilities|Array|FindItem (Variables|AI|GetSquad) self))
  (for _array_element (Variables|AI|GetSquad)
    (Variables|BP_DummyEnemy_C|SetSquad _array_element (Variables|AI|GetSquad)))
  (Actor|DestroyActor (Variables|Ressources|GetWeapon))
  (Actor|DestroyActor))