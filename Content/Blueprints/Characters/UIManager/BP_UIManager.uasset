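; BP_UIManager creates and controls the player's screen widgets: HUD, choice, pause, options, highscore and death screens.
; On BeginPlay it builds all but the death screen, showing only the HUD and cross-linking the pause, options and highscore widgets for menu navigation.
; Pause, ChoiceUI (which passes in two choice names) and SetDead (which spawns the death screen) each pause the game and switch to cursor-driven UI-only input.
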(event Custom|Pause
  (bind _pausescreen (Variables|Default|GetPausescreen))
  (Variables|/Script/Engine.PlayerController|SetbShowMouseCursor (Game|GetPlayerController 0) true)
  (Game|SetGamePaused true)
  (Widget|SetVisibility _pausescreen "Visible")
  (Input|SetInputModeUIOnly (Game|GetPlayerController 0) _pausescreen "DoNotLock")
  (Widget|SetVisibility (Variables|Default|GetMainHud) "Hidden"))

(event EventBeginPlay
  (CallFunction|HudSetUp)
  (CallFunction|Start))

(fn ConstructionScript)

(fn HudSetUp
  (bind _returnvalue (Game|GetPlayerController 0))
  (bind _returnvalue_2 (UserInterface|CreateWidget "/Game/Blueprints/Hud/WBP_Hud_V1.WBP_Hud_V1_C" _returnvalue))
  (bind _output_get (Variables|Default|SetMainHud _returnvalue_2))
  (UserInterface|Viewport|AddtoViewport _output_get 0)
  (bind _returnvalue_3 (UserInterface|CreateWidget "/Game/Blueprints/Hud/WBP_ChoiceScreen.WBP_ChoiceScreen_C" _returnvalue))
  (bind _output_get_2 (Variables|Default|SetChoiceScreen _returnvalue_3))
  (UserInterface|Viewport|AddtoViewport _output_get_2 0)
  (Widget|SetVisibility _output_get_2 "Hidden"))

(fn SetDead
  (bind _returnvalue (UserInterface|CreateWidget "/Game/Blueprints/Hud/WBP_DeathScreen_V1.WBP_DeathScreen_V1_C"))
  (UserInterface|Viewport|AddtoViewport _returnvalue 0)
  (Variables|/Script/Engine.PlayerController|SetbShowMouseCursor (Game|GetPlayerController 0) true)
  (Game|SetGamePaused true)
  (Input|SetInputModeUIOnly (Game|GetPlayerController 0) _returnvalue "DoNotLock"))

(fn Start
  (bind _returnvalue (Game|GetPlayerController 0))
  (bind _returnvalue_2 (UserInterface|CreateWidget "/Game/Blueprints/Hud/WBP_PauseScreen.WBP_PauseScreen_C" _returnvalue))
  (bind _output_get (Variables|Default|SetPausescreen _returnvalue_2))
  (UserInterface|Viewport|AddtoViewport _returnvalue_2 0)
  (Widget|SetVisibility _output_get "Hidden")
  (bind _returnvalue_3 (UserInterface|CreateWidget "/Game/Blueprints/Hud/WBP_Options.WBP_Options_C" _returnvalue))
  (bind _output_get_2 (Variables|Default|SetOptions _returnvalue_3))
  (UserInterface|Viewport|AddtoViewport _returnvalue_3 0)
  (Widget|SetVisibility _returnvalue_3 "Hidden")
  (bind _returnvalue_4 (UserInterface|CreateWidget "/Game/Blueprints/Hud/WBP_Highscore.WBP_Highscore_C" _returnvalue))
  (bind _output_get_3 (Variables|Default|SetHighscore _returnvalue_4))
  (UserInterface|Viewport|AddtoViewport _output_get_3 0)
  (Widget|SetVisibility _output_get_3 "Hidden")
  (Variables|/Game/Blueprints/Hud/WBP_PauseScreen.WBP_PauseScreen_C|SetMainHud (Variables|Default|GetPausescreen) (Variables|Default|GetMainHud))
  (Variables|/Game/Blueprints/Hud/WBP_PauseScreen.WBP_PauseScreen_C|SetOptions (Variables|Default|GetPausescreen) (Variables|Default|GetOptions))
  (Variables|/Game/Blueprints/Hud/WBP_Options.WBP_Options_C|SetMainMenu (Variables|Default|GetOptions) (Variables|Default|GetPausescreen))
  (Variables|/Game/Blueprints/Hud/WBP_Highscore.WBP_Highscore_C|SetMainMenu (Variables|Default|GetHighscore) (Variables|Default|GetPausescreen))
  (Variables|/Game/Blueprints/Hud/WBP_PauseScreen.WBP_PauseScreen_C|SetHighscore (Variables|Default|GetPausescreen) (Variables|Default|GetHighscore)))

(fn ChoiceUI
  (params (Choice1 :type Integer) (Choice2 :type Integer))
  (bind _returnvalue (Game|GetPlayerController 0))
  (bind _choicescreen (Variables|Default|GetChoiceScreen))
  (Widget|SetVisibility _choicescreen "Visible")
  (Variables|/Game/Blueprints/Hud/WBP_ChoiceScreen.WBP_ChoiceScreen_C|SetName1 _choicescreen Choice1)
  (Variables|/Game/Blueprints/Hud/WBP_ChoiceScreen.WBP_ChoiceScreen_C|SetName2 _choicescreen Choice2)
  (Game|SetGamePaused true)
  (Variables|/Script/Engine.PlayerController|SetbShowMouseCursor _returnvalue true)
  (Input|SetInputModeUIOnly _returnvalue _choicescreen "DoNotLock"))