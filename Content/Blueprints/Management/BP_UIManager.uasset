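; UI manager that owns the player's HUD and handles the pause, options, highscore and death screens.
; On BeginPlay it adds the HUD and the hidden menu widgets to the viewport, then cross-links the menus by reference.
; Pause and SetDead halt the game and switch to cursor-driven UI input, hiding or removing the HUD respectively; the death screen is created on demand.
; A perk/ability-learned event is forwarded to the HUD.
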(event Custom|Pause
  (bind _pausescreen (Variables|Default|GetPausescreen))
  (Variables|/Script/Engine.PlayerController|SetbShowMouseCursor (Game|GetPlayerController 0) true)
  (Game|SetGamePaused true)
  (Widget|SetVisibility _pausescreen "Visible")
  (Input|SetInputModeUIOnly (Game|GetPlayerController 0) _pausescreen "DoNotLock")
  (Widget|SetVisibility (Variables|Default|GetMainHud) "Hidden"))

(event Custom|NewPerk/AbilityLearned
  (Default|Perk/AbilityGained (Variables|Default|GetMainHud)))

(event EventBeginPlay
  (CallFunction|HudSetUp)
  (CallFunction|Start))

(fn ConstructionScript)

(fn HudSetUp
  (bind _returnvalue (UserInterface|CreateWidget "/Game/Blueprints/UI/WBP_HUD.WBP_HUD_C" (Game|GetPlayerController 0)))
  (bind _output_get (Variables|Default|SetMainHud _returnvalue))
  (UserInterface|Viewport|AddtoViewport _output_get 0))

(fn SetDead
  (bind _returnvalue (UserInterface|CreateWidget "/Game/Blueprints/UI/WBP_DeathScreen.WBP_DeathScreen_C"))
  (UserInterface|Viewport|AddtoViewport _returnvalue 0)
  (Variables|/Script/Engine.PlayerController|SetbShowMouseCursor (Game|GetPlayerController 0) true)
  (Game|SetGamePaused true)
  (CallFunction|RemoveHud)
  (Input|SetInputModeUIOnly (Game|GetPlayerController 0) _returnvalue "DoNotLock"))

(fn Start
  (bind _returnvalue (Game|GetPlayerController 0))
  (bind _returnvalue_2 (UserInterface|CreateWidget "/Game/Blueprints/UI/WBP_PauseScreen.WBP_PauseScreen_C" _returnvalue))
  (bind _output_get (Variables|Default|SetPausescreen _returnvalue_2))
  (UserInterface|Viewport|AddtoViewport _returnvalue_2 0)
  (Widget|SetVisibility _output_get "Hidden")
  (bind _returnvalue_3 (UserInterface|CreateWidget "/Game/Blueprints/UI/WBP_Options.WBP_Options_C" _returnvalue))
  (bind _output_get_2 (Variables|Default|SetOptions _returnvalue_3))
  (UserInterface|Viewport|AddtoViewport _output_get_2 0)
  (Widget|SetVisibility _output_get_2 "Hidden")
  (bind _returnvalue_4 (UserInterface|CreateWidget "/Game/Blueprints/UI/WBP_Highscore.WBP_Highscore_C" _returnvalue))
  (bind _output_get_3 (Variables|Default|SetHighscore _returnvalue_4))
  (UserInterface|Viewport|AddtoViewport _output_get_3 0)
  (Widget|SetVisibility _output_get_3 "Hidden")
  (Variables|/Game/Blueprints/UI/WBP_PauseScreen.WBP_PauseScreen_C|SetMainHud (Variables|Default|GetPausescreen) (Variables|Default|GetMainHud))
  (Variables|/Game/Blueprints/UI/WBP_PauseScreen.WBP_PauseScreen_C|SetOptions (Variables|Default|GetPausescreen) (Variables|Default|GetOptions))
  (Variables|/Game/Blueprints/UI/WBP_Options.WBP_Options_C|SetMainMenu (Variables|Default|GetOptions) (Variables|Default|GetPausescreen))
  (Variables|/Game/Blueprints/UI/WBP_Highscore.WBP_Highscore_C|SetMainMenu (Variables|Default|GetHighscore) (Variables|Default|GetPausescreen))
  (Variables|/Game/Blueprints/UI/WBP_PauseScreen.WBP_PauseScreen_C|SetHighscore (Variables|Default|GetPausescreen) (Variables|Default|GetHighscore)))

(fn NewFunction0)

(fn RemoveHud
  (bind _foundwidgets (Widget|GetAllWidgetsOfClass "/Game/Blueprints/UI/WBP_HUD.WBP_HUD_C" false))
  (Widget|RemovefromParent _foundwidgets))