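; Arena manager that locks the player into a spawner arena and cleanses it once every spawner is removed.
; Entering the Box trigger, sized from Triggerrange in construction, makes the barriers visible and blocking on a custom collision channel.
; It hands itself to each spawner on BeginPlay and exposes RemoveObject to shrink the list.
; Tick polls for an empty list, then once activates the shrine, cleanses the fog, starts ArenaCleanse and destroys the barriers.
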(event OnComponentBeginOverlap(Box)
  (params (OverlappedComponent :type Primitive%20Component%20Object%20Reference) (OtherActor :type Actor%20Object%20Reference) (OtherComp :type Primitive%20Component%20Object%20Reference) (OtherBodyIndex :type Integer) (bFromSweep :type Boolean) (SweepResult :type Hit%20Result%20Structure%20%28by%20ref%29))
  (Utilities|Casting|CastToBP_MainCharacter OtherActor)
  (for _array_element (Variables|ArenaComponents|GetBarrier)
    (Utilities|IsValid _array_element
      (:Is%20Valid
        (Rendering|SetVisibility (Variables|/Game/Blueprints/LevelGenerator/Arena/BP_Barrier.BP_Barrier_C|GetCube _array_element) true false)
        (Collision|SetCollisionResponsetoChannel (Variables|/Game/Blueprints/LevelGenerator/Arena/BP_Barrier.BP_Barrier_C|GetCube _array_element) "ECC_GameTraceChannel2" "ECR_Block")))))

(event EventBeginPlay
  (for _array_element (Variables|ArenaComponents|GetSpawners)
    (Variables|/Game/Blueprints/LevelGenerator/Spawners/BP_EnemySpawn.BP_EnemySpawn_C|SetArenaManager _array_element self)))

(event EventTick
  (params (DeltaSeconds :type Float%20%28single-precision%29))
  (if (and (<= (Utilities|Array|Length (Variables|ArenaComponents|GetSpawners)) 0) (Variables|Default|Getnotcleansed))
    (Variables|Default|Setnotcleansed false)
    (Default|EventActivateShrine (Variables|ArenaComponents|GetArenaShrine))
    (for _array_element (Variables|ArenaComponents|GetArenaFog)
      (Default|EventCleansed _array_element))
    (Default|EventStartCleanse (Variables|ArenaComponents|GetArenaCleanse))
    (for _array_element_2 (Variables|ArenaComponents|GetBarrier)
      (Utilities|IsValid _array_element_2
        (:Is%20Valid
          (Actor|DestroyActor _array_element_2))))))

(fn ConstructionScript
  (Components|Box|SetBoxExtent (Variables|Default|GetBox) (Variables|Components|GetTriggerrange) true))

(fn RemoveObject
  (params (Spawner :type BP%20Enemy%20Spawn%20Object%20Reference))
  (bind _spawners (Variables|ArenaComponents|GetSpawners))
  (Utilities|Array|RemoveIndex _spawners (Utilities|Array|FindItem _spawners Spawner)))