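; BP_GameManager spawns and possesses the main character, spawns the UI manager, and hands out random abilities and perks to the player.
; On BeginPlay it registers both managers with the player and copies the full ability and perk lists into learnable pools.
; Random abilities leave the pool once learned, falling back to random, repeatable perks when none remain.
; Abilities set learned flags on the player, while perks adjust player stats, each with a printed message.
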(event EventBeginPlay
  (Player|SpawnPlayer)
  (UI|SpawnUI)
  (Player|SetupListOfAbilities)
  (Player|SetupListOfPerks))

(fn ConstructionScript)

(fn SetAttributes
  (params (Values :type Balancing%20Values%20Att%20Structure))
  (Variables|Player|SetPlayerAtrributes Values))

(fn SetCombat
  (params (Values :type Balancing%20Values%20Combat%20Structure))
  (Variables|Player|SetPlayerCombat Values))

(fn SetAbilities
  (params (Values :type Balancing%20Values%20Abilities%20Structure))
  (Variables|Player|SetPlayerAbilities Values))

(fn SpawnUI
  (bind _returnvalue (Game|SpawnActorfromClass "/Game/Blueprints/Management/BP_UIManager.BP_UIManager_C" (Transformation|GetActorTransform) "Undefined" 0 0))
  (Default|RegisterUIManager (Variables|Player|GetPlayer) _returnvalue))

(fn SpawnPlayer
  (bind _returnvalue (Game|SpawnActorfromClass "/Game/Blueprints/Characters/MainCharacter/BP_MainCharacter.BP_MainCharacter_C" (Transformation|GetActorTransform) "AdjustIfPossibleButAlwaysSpawn" 0 0))
  (Variables|Player|SetPlayer _returnvalue)
  (Default|RegisterGameManager _returnvalue self)
  (Pawn|Possess (Game|GetPlayerController 0) _returnvalue))

(fn SetupListOfAbilities
  (for _array_element (Variables|Player|GetAllAbilities)
    (Utilities|Array|Add (Variables|Player|GetLearnableAbilities) _array_element)))

(fn AddRandomAbilitytoPlayer
  (bind _learnableabilities (Variables|Player|GetLearnableAbilities))
  (bind _returnvalue (Utilities|Array|Length _learnableabilities))
  (if (> _returnvalue 0)
    (bind _output_get (LocalVariables|SetIndex (Math|Random|RandomIntegerinRange 0 (- _returnvalue 1))))
    (LocalVariables|SetChoice (Utilities|Array|Get(acopy) (Variables|Player|GetLearnableAbilities) _output_get))
    (Utilities|Array|RemoveIndex (Variables|Player|GetLearnableAbilities) _output_get)
    (Player|ApplyAbilitytoPlayer (LocalVariables|GetChoice))
    (else
      (Player|AddRandomPerktoPlayer))))

(fn SetupListOfPerks
  (for _array_element (Variables|Player|GetAllPerks)
    (Utilities|Array|Add (Variables|Player|GetLearnablePerks) _array_element)))

(fn AddRandomPerktoPlayer
  (bind _learnableperks (Variables|Player|GetLearnablePerks))
  (bind _returnvalue (Utilities|Array|Length _learnableperks))
  (if (> _returnvalue 0)
    (Player|ApplyPerktoPlayer (Utilities|Array|Get(acopy) (Variables|Player|GetLearnablePerks) (Math|Random|RandomIntegerinRange 0 (- _returnvalue 1))))))

(fn ApplyPerktoPlayer
  (params (Perk :type Perks%20Enum :default "NewEnumerator0"))
  (bind _player (Variables|Player|GetPlayer))
  (switch Utilities|FlowControl|Switch|SwitchonPerks Perk
    (:NewEnumerator0
      (Variables|/Game/Blueprints/Characters/MainCharacter/BP_MainCharacter.BP_MainCharacter_C|SetRageMultiplier _player (* (Variables|/Game/Blueprints/Characters/MainCharacter/BP_MainCharacter.BP_MainCharacter_C|GetRageMultiplier _player) (Variables|PerkMods|GetRageGrowth)))
      (Development|PrintString "Rage Gain +20%"))
    (:NewEnumerator1
      (Variables|/Game/Blueprints/Characters/MainCharacter/BP_MainCharacter.BP_MainCharacter_C|SetRageDecayMultiplier _player (* (Variables|/Game/Blueprints/Characters/MainCharacter/BP_MainCharacter.BP_MainCharacter_C|GetRageDecayMultiplier _player) (Variables|PerkMods|GetRageDecay)))
      (Development|PrintString "Rage Decay -20%"))
    (:NewEnumerator2
      (Variables|/Game/Blueprints/Characters/MainCharacter/BP_MainCharacter.BP_MainCharacter_C|SetmaxHealth _player (+ (Variables|/Game/Blueprints/Characters/MainCharacter/BP_MainCharacter.BP_MainCharacter_C|GetmaxHealth _player) (Variables|PerkMods|GetMaxHP)))
      (Development|PrintString "Max HP +20"))
    (:NewEnumerator3
      (Variables|/Game/Blueprints/Characters/MainCharacter/BP_MainCharacter.BP_MainCharacter_C|SetDodgeCooldownTime _player (* (Variables|/Game/Blueprints/Characters/MainCharacter/BP_MainCharacter.BP_MainCharacter_C|GetDodgeCooldownTime _player) (Variables|PerkMods|GetDodgeCDR)))
      (Development|PrintString "Dodge Cooldown -20%"))
    (:NewEnumerator4
      (Variables|/Game/Blueprints/Characters/MainCharacter/BP_MainCharacter.BP_MainCharacter_C|SetBaseHealChance _player (+ (Variables|/Game/Blueprints/Characters/MainCharacter/BP_MainCharacter.BP_MainCharacter_C|GetBaseHealChance _player) (Variables|PerkMods|GetHealchance)))
      (Development|PrintString "Chance to heal +10%"))
    (:NewEnumerator5
      (Variables|/Game/Blueprints/Characters/MainCharacter/BP_MainCharacter.BP_MainCharacter_C|SetEXPMultiplier _player (* (Variables|/Game/Blueprints/Characters/MainCharacter/BP_MainCharacter.BP_MainCharacter_C|GetEXPMultiplier _player) (Variables|PerkMods|GetEXPGain)))
      (Development|PrintString "EXP Gain +20%"))
    (:NewEnumerator6
      (Variables|/Game/Blueprints/Characters/MainCharacter/BP_MainCharacter.BP_MainCharacter_C|SetOutofCombatDuration _player (* (Variables|/Game/Blueprints/Characters/MainCharacter/BP_MainCharacter.BP_MainCharacter_C|GetOutofCombatDuration _player) (Variables|PerkMods|GetEnrageTime)))
      (Development|PrintString "Enraged +0.2sec"))
    (:NewEnumerator7
      (Variables|/Game/Blueprints/Characters/MainCharacter/BP_MainCharacter.BP_MainCharacter_C|SetCooldownMultiplier _player (* (Variables|/Game/Blueprints/Characters/MainCharacter/BP_MainCharacter.BP_MainCharacter_C|GetCooldownMultiplier _player) (Variables|PerkMods|GetPowerCDR)))
      (Development|PrintString "Ability Cooldowns -20%"))))

(fn ApplyAbilitytoPlayer
  (params (Ability :type Ability%20Enum :default "NewEnumerator0"))
  (bind _player (Variables|Player|GetPlayer))
  (switch Utilities|FlowControl|Switch|SwitchonAbility Ability
    (:NewEnumerator0
      (Variables|/Game/Blueprints/Characters/MainCharacter/BP_MainCharacter.BP_MainCharacter_C|SetSpinLearned _player true)
      (Development|PrintString "Spin Learned!"))
    (:NewEnumerator1
      (Variables|/Game/Blueprints/Characters/MainCharacter/BP_MainCharacter.BP_MainCharacter_C|SetLeapLearned _player true)
      (Development|PrintString "Leap Learned!"))
    (:NewEnumerator2
      (Variables|/Game/Blueprints/Characters/MainCharacter/BP_MainCharacter.BP_MainCharacter_C|SetChargeLearned _player true)
      (Development|PrintString "Charge Learned!"))
    (:NewEnumerator3
      (Variables|/Game/Blueprints/Characters/MainCharacter/BP_MainCharacter.BP_MainCharacter_C|SetShoutLearned _player true)
      (Development|PrintString "Shout Learned!"))))