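; BP_HealOrb is a healing pickup projectile that seeks out the player and restores health on contact.
; On BeginPlay it turns on homing in its ProjectileMovement, targeting the capsule of the player's BP_MainCharacter with a strong acceleration.
; When its Sphere overlaps a BP_MainCharacter, it passes its Healing amount to ChangeHealth and destroys itself.
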(event OnComponentBeginOverlap(Sphere)
  (params (OverlappedComponent :type Primitive%20Component%20Object%20Reference) (OtherActor :type Actor%20Object%20Reference) (OtherComp :type Primitive%20Component%20Object%20Reference) (OtherBodyIndex :type Integer) (bFromSweep :type Boolean) (SweepResult :type Hit%20Result%20Structure%20%28by%20ref%29))
  (bind _asbp_main_character (Utilities|Casting|CastToBP_MainCharacter OtherActor))
  (Default|ChangeHealth _asbp_main_character (Variables|Default|GetHealing))
  (Actor|DestroyActor))

(event EventBeginPlay
  (bind _projectilemovement (Variables|Default|GetProjectileMovement))
  (bind _asbp_main_character (Utilities|Casting|CastToBP_MainCharacter (Game|GetPlayerCharacter 0)))
  (Variables|/Script/Engine.ProjectileMovementComponent|SetbIsHomingProjectile _projectilemovement true)
  (Variables|/Script/Engine.ProjectileMovementComponent|SetHomingAccelerationMagnitude _projectilemovement 9e+03)
  (Variables|/Script/Engine.ProjectileMovementComponent|SetHomingTargetComponent _projectilemovement (Variables|/Script/Engine.Character|GetCapsuleComponent _asbp_main_character)))

(fn ConstructionScript)